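; BP_IBCharacterPlayer is the player character Blueprint, with number-key shortcuts for assigning roles to AI characters.
; Keys 1 to 4 pass the default, construction, scientist or guard role to Set Role.
; Set Role gathers all BP_IBCharacterAI actors but returns inside the loop, so only the first one found receives the role.
; BeginPlay adds a fixed health bonus to the player, printing health before and after.
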(event `Key|Four`
  (params (Key :type "Key Structure"))
  (:`Pressed`
    (`self.Set Role` "GUARD")))

(event `Key|Three`
  (params (Key :type "Key Structure"))
  (:`Pressed`
    (`self.Set Role` "SCIENTIST")))

(event `Key|Two`
  (params (Key :type "Key Structure"))
  (:`Pressed`
    (`self.Set Role` "CONSTRUCTION")))

(event `Key|One`
  (params (Key :type "Key Structure"))
  (:`Pressed`
    (`self.Set Role` "DEFAULT")))

(event `self.ReceiveBeginPlay`
  (bind _returnvalue (`self.GetHealth`))
  (bind _returnvalue_2 (`KismetStringLibrary.Conv_IntToString` _returnvalue))
  (`KismetSystemLibrary.PrintString` _returnvalue_2)
  (`self.SetHealth` (+ _returnvalue 50))
  (`KismetSystemLibrary.PrintString` _returnvalue_2))

(event `self.ReceiveTick`
  (params (DeltaSeconds :type "Float (single-precision)")))

(fn `UserConstructionScript`)
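; BP_IBCharacterAI is an AI character with a switchable role of guard, construction or scientist.
; When pawn sensing sees an IBCharacterPlayer, it moves to a point offset along world X from the player's location.
; SetCharacterRole swaps the body material to match the role, falling back to the default, then logs and stores the role.
; Tick prints the current role every frame as debug output.
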(event `self.PawnSensing.OnSeePawn`
  (params (Pawn :type "Pawn Object Reference"))
  (bind _asibcharacter_player (cast `IBCharacterPlayer` Pawn))
  (`|AIMoveTo` self (`KismetMathLibrary.MakeVector` (- (.x (`self.K2_GetActorLocation` _asibcharacter_player)) 200.0) (.y (`self.K2_GetActorLocation` _asibcharacter_player)) (.z (`self.K2_GetActorLocation` _asibcharacter_player))) null))

(event `self.ReceiveBeginPlay`)

(event `self.ReceiveTick`
  (params (DeltaSeconds :type "Float (single-precision)"))
  (`KismetSystemLibrary.PrintString` (`self.GetRole`)))

(fn `SetCharacterRole`
  (params (Role :type String :default "DEFAULT") (Name :type String))
  (bind _mesh (`self.Mesh`))
  (if (`KismetStringLibrary.EqualEqual_StrStr` Role "GUARD")
    (`PrimitiveComponent.SetMaterial` _mesh 0 "/Game/Character/Materials/M_UE4Man_Body_AI_Guard.M_UE4Man_Body_AI_Guard")
    (elif (`KismetStringLibrary.EqualEqual_StrStr` Role "CONSTRUCTION")
      (`PrimitiveComponent.SetMaterial` _mesh 0 "/Game/Character/Materials/M_UE4Man_Body_AI_Construction.M_UE4Man_Body_AI_Construction")
      (elif (`KismetStringLibrary.EqualEqual_StrStr` Role "SCIENTIST")
        (`PrimitiveComponent.SetMaterial` _mesh 0 "/Game/Character/Materials/M_UE4Man_Body_AI_Science.M_UE4Man_Body_AI_Science")
        (else
          (`PrimitiveComponent.SetMaterial` _mesh 0 "/Game/Character/Materials/M_UE4Man_Body.M_UE4Man_Body")))))
  (`KismetSystemLibrary.PrintString` (`KismetStringLibrary.Concat_StrStr` (`KismetStringLibrary.Concat_StrStr` Name "switched roles to ") Role) false)
  (`self.SetRole` Role))

(fn `UserConstructionScript`)